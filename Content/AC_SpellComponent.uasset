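; Actor component that casts Harry Potter-style spells (Flipendo, Alohomora) on a target and shows the spell name on screen.
; ApplySpell stores the current spell, displays its name in a viewport widget and restarts a timer that clears it after a delay.
; It then casts the target by spell type: Flipendo makes turtle receivers or enemies vulnerable, while Alohomora unlocks Alohomora lockers.
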(event `HideSpellLater`
  (`KismetSystemLibrary.K2_ClearAndInvalidateTimerHandle` (`self.HideTimer`))
  (bind _returnvalue (`KismetSystemLibrary.K2_SetTimerDelegate` (delegate `HideSpell`) (`self.DisplayTime`)))
  (set `self.HideTimer` _returnvalue))

(event `HideSpell`
  (set `self.CurrentSpell` "NewEnumerator0")
  (`/Game/UI/WBP_SpellDisplay.SetSpellText` (`self.SpellWidget`) ""))

(event `CustomEvent`
  (bind _returnvalue (`|CreateWidget` (`self.SpellWidgetClass`) (`GameplayStatics.GetPlayerController` 0)))
  (set `self.SpellWidget` _returnvalue)
  (`UserWidget.AddToViewport` (`self.SpellWidget`) 0))

(fn `ApplySpell`
  (params (Spell :type "/Game/Blueprints/Enums/E_Spell Enum" :default "NewEnumerator0") (Target :type "Actor Object Reference"))
  (set `self.CurrentSpell` Spell)
  (`/Game/UI/WBP_SpellDisplay.SetSpellText` (`self.SpellWidget`) (`self.GetSpellName` Spell))
  (`self.HideSpellLater`)
  (switch `/Game/Blueprints/Enums/E_Spell` Spell
    (:`NewEnumerator1`
      (bind _asbp_turtle_spell_receiver (cast `/Game/Blueprints/HP_BPs/BP_TurtleSpellReceiver` Target)
        (:`then`
          (`/Game/Blueprints/HP_BPs/BP_TurtleSpellReceiver.SetVulnerable` _asbp_turtle_spell_receiver))
        (:`CastFailed`
          (bind _asbp_enemy (cast `/Game/Blueprints/HP_BPs/Enemy/BP_Enemy` (`local.Target`)))
          (`/Game/Blueprints/HP_BPs/Enemy/BP_Enemy.SetVulnerable` _asbp_enemy))))
    (:`NewEnumerator2`
      (bind _asbp_locker_alohomora (cast `/Game/Blueprints/HP_BPs/BP_LockerAlohomora` Target))
      (set `/Game/Blueprints/HP_BPs/BP_LockerAlohomora.IsUnlocked` true _asbp_locker_alohomora))))

(fn `GetSpellName`
  (params (Spell :type "/Game/Blueprints/Enums/E_Spell Enum" :default "NewEnumerator0"))
  (returns (Name :type Text))
  (switch `/Game/Blueprints/Enums/E_Spell` Spell
    (:`NewEnumerator0`
      (return ""))
    (:`NewEnumerator1`
      (return "¡Flipendo!"))
    (:`NewEnumerator2`
      (return "¡Alohomora!"))))