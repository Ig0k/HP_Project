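; BP_Enemy is an enemy that feeds AI perception into its Blackboard and can be pushed.
; Perception updates write IsPlayerInSight and TargetActor to the AIController's Blackboard, without checking that the sensed actor is the player.
; Tick applies a timed push, moving the actor along PushDirection by PushForce, without sweep, until PushCurrentTime reaches PushMaxTime.
; An AIMoveTo node is left unconnected and never runs.
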(event `self.ReceiveBeginPlay`)

(event `self.ReceiveTick`
  (params (DeltaSeconds :type "Float (single-precision)"))
  (if (< (`self.PushCurrentTime`) (`self.PushMaxTime`))
    (`|ExecutionSequence`
      (:`then_0`
        (`self.K2_SetActorLocation` (+ (`self.K2_GetActorLocation`) (* (* (`self.PushDirection`) (`self.PushForce`)) DeltaSeconds))))
      (:`then_1`
        (if (< (`self.PushCurrentTime`) (`self.PushMaxTime`))
          (set `self.PushCurrentTime` (+ (`self.PushCurrentTime`) DeltaSeconds)))))))

(event `self.AIPerception.OnTargetPerceptionUpdated`
  (params (Actor :type "Actor Object Reference") (Stimulus :type "AIStimulus Structure"))
  (bind _asaicontroller (cast `AIController` (`self.GetController`)))
  (bind _returnvalue (`AIBlueprintHelperLibrary.GetBlackboard` _asaicontroller))
  (`BlackboardComponent.SetValueAsBool` _returnvalue "IsPlayerInSight" (`.bSuccessfullySensed` (break `AIStimulus` Stimulus)))
  (`BlackboardComponent.SetValueAsObject` _returnvalue "TargetActor" Actor))

(fn `UserConstructionScript`)