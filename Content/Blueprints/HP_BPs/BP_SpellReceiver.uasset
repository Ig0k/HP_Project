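; BP_SpellReceiver is a block that slides when pushed, apparently by the Flipendo spell, up to a limited number of pushes.
; While CanMove is set, Tick plays a sound once, then uses MoveDirectionState to select one of four duplicated collapsed graphs.
; Each moves the actor unswept along its forward or right axis until PushDuration elapses, then stops and increments the push count.
; Nothing here sets CanMove true or chooses the direction.
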(event `self.ReceiveTick`
  (params (DeltaSeconds :type "Float (single-precision)"))
  (if (< (`self.currentPushes`) (`self.MaxPushes`))
    (if (`self.CanMove`)
      (`|ExecutionSequence`
        (:`then_0`
          (if (not (`self.SoundPlayed`))
            (`GameplayStatics.PlaySoundAtLocation` "/Game/Sounds/BlockMoveFlipendoSFX.BlockMoveFlipendoSFX" (`self.K2_GetActorLocation` self) (struct) 0.6 1.0 0.0 null null null null)
            (set `self.SoundPlayed` true)))
        (:`then_1`
          (switch `/Game/Blueprints/Enums/Enum_SpellReciever_MoveDir` (`self.MoveDirectionState`)
            (:`NewEnumerator0`
              (`self.K2_SetActorLocation` (+ (`self.K2_GetActorLocation`) (* (* (`self.GetActorForwardVector`) (`self.PushForce`)) DeltaSeconds)))
              (bind _output_get (set `self.pushCD` (+ (`self.pushCD`) (`GameplayStatics.GetWorldDeltaSeconds`))))
              (if (>= _output_get (`self.PushDuration`))
                (set `self.CanMove` false)
                (if (< (`self.currentPushes`) (`self.MaxPushes`))
                  (set `self.currentPushes` (+ (`self.currentPushes`) 1))
                  (set `self.pushCD` 0.0)
                  (set `self.SoundPlayed` false))))
            (:`NewEnumerator1`
              (`self.K2_SetActorLocation` (+ (`self.K2_GetActorLocation`) (* (* (`KismetMathLibrary.NegateVector` (`self.GetActorForwardVector`)) (`self.PushForce`)) DeltaSeconds)))
              (bind _output_get_2 (set `self.pushCD` (+ (`self.pushCD`) (`GameplayStatics.GetWorldDeltaSeconds`))))
              (if (>= _output_get_2 (`self.PushDuration`))
                (set `self.CanMove` false)
                (if (< (`self.currentPushes`) (`self.MaxPushes`))
                  (set `self.currentPushes` (+ (`self.currentPushes`) 1))
                  (set `self.pushCD` 0.0)
                  (set `self.SoundPlayed` false))))
            (:`NewEnumerator2`
              (`self.K2_SetActorLocation` (+ (`self.K2_GetActorLocation`) (* (* (`self.GetActorRightVector`) (`self.PushForce`)) DeltaSeconds)))
              (bind _output_get_3 (set `self.pushCD` (+ (`self.pushCD`) (`GameplayStatics.GetWorldDeltaSeconds`))))
              (if (>= _output_get_3 (`self.PushDuration`))
                (set `self.CanMove` false)
                (if (< (`self.currentPushes`) (`self.MaxPushes`))
                  (set `self.currentPushes` (+ (`self.currentPushes`) 1))
                  (set `self.pushCD` 0.0)
                  (set `self.SoundPlayed` false))))
            (:`NewEnumerator3`
              (`self.K2_SetActorLocation` (+ (`self.K2_GetActorLocation`) (* (* (`KismetMathLibrary.NegateVector` (`self.GetActorRightVector`)) (`self.PushForce`)) DeltaSeconds)))
              (bind _output_get_4 (set `self.pushCD` (+ (`self.pushCD`) (`GameplayStatics.GetWorldDeltaSeconds`))))
              (if (>= _output_get_4 (`self.PushDuration`))
                (set `self.CanMove` false)
                (if (< (`self.currentPushes`) (`self.MaxPushes`))
                  (set `self.currentPushes` (+ (`self.currentPushes`) 1))
                  (set `self.pushCD` 0.0)
                  (set `self.SoundPlayed` false))))))))))

(fn `UserConstructionScript`)