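; BP_ProjectileSpawner is an actor that periodically fires a volley of BP_Projectile actors from its own location.
; Tick accumulates delta time up to ShootCooldown, then spawns one scaled-down projectile per yaw in BulletsRotationz at a configurable Z offset.
; The yaws are world-space, independent of the spawner's rotation.
; The timer resets inside the spawn loop, so an empty rotation array stops the cycle after the first cooldown.
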(event `self.ReceiveTick`
  (params (DeltaSeconds :type "Float (single-precision)"))
  (bind (_returnvalue_x _returnvalue_y _returnvalue_z) (`KismetMathLibrary.BreakVector` (`self.K2_GetActorLocation`)))
  (if (< (`self.CurrentCooldown`) (`self.ShootCooldown`))
    (set `self.CurrentCooldown` (+ DeltaSeconds (`self.CurrentCooldown`)))
    (if (>= (`self.CurrentCooldown`) (`self.ShootCooldown`))
      (bind _output_get (set `self.SpawnPosition` (`KismetMathLibrary.MakeVector` _returnvalue_x _returnvalue_y (+ (`self.ZOffsetSpawn`) _returnvalue_z))))
      (for _array_element (`self.BulletsRotationz`)
        (`|SpawnActorFromClass` "/Game/Blueprints/HP_BPs/BP_Projectile.BP_Projectile_C" (`KismetMathLibrary.MakeTransform` _output_get (`KismetMathLibrary.MakeRotator` 0.0 0.0 _array_element) (0.75 0.75 0.75)) "Undefined" "MultiplyWithRoot" null null)
        (set `self.CurrentCooldown` 0.0)))))

(fn `UserConstructionScript`)