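; Older turtle spell receiver actor that can be shoved by Flipendo while it is off a pressure plate.
; Tick sweeps it along PushDirection for a timed push while CanMove is set, counting pushes up to a limit and refreshing direction from SetPushDir.
; When Flipendo is not usable, Tick forces a fixed rotation instead.
; SetVulnerableAlpha drives a material parameter on its dynamic materials; SetVectorMove is an empty stub.
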(event `self.ReceiveTick`
  (params (DeltaSeconds :type "Float (single-precision)"))
  (if (`self.IsOnPressurePlate`)
    _
    (elif (`self.CanUseFlipendo`)
      (if (< (`self.currentPushes`) (`self.MaxPushes`))
        (if (`self.CanMove`)
          (set `self.CanObtainPlayerForward` true)
          (`|ExecutionSequence`
            (:`then_0`
              (`self.K2_SetActorLocation` (+ (`self.K2_GetActorLocation`) (* (* (stale _output_get_2) (`self.PushForce`)) DeltaSeconds)) true)
              (bind _output_get (set `self.pushCD` (+ (`self.pushCD`) (`GameplayStatics.GetWorldDeltaSeconds`))))
              (if (>= _output_get (`self.PushDuration`))
                (set `self.CanMove` false)
                (if (< (`self.currentPushes`) (`self.MaxPushes`))
                  (set `self.currentPushes` (+ (`self.currentPushes`) 1))
                  (set `self.pushCD` 0.0))))
            (:`then_1`
              (if (`self.CanObtainPlayerForward`)
                (bind _output_get_2 (set `self.PushDirection` (`self.SetPushDir`)))))
            (:`then_2`
              (set `self.CanObtainPlayerForward` false)))))
      (else
        (`self.K2_SetActorRotation` (struct :`Pitch` 180.0 :`Yaw` 180.0 :`Roll` 180.0))))))

(fn `SetVectorMove`
  (params (InputVector :type "Vector Structure")))

(fn `SetVulnerableAlpha`
  (params (Alpha :type "Float (double-precision)"))
  (for _array_element (`self.DynMats`)
    (`MaterialInstanceDynamic.SetScalarParameterValue` _array_element "VulnerableAlpha" (`local.Alpha`))))

(fn `UserConstructionScript`)