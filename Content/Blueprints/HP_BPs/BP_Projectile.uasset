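; BP_Projectile is a projectile that flies forward and damages actors it overlaps.
; Tick moves it along its forward vector by PushForce without sweep or a movement component, and destroys it once its accumulated DestroyCooldown reaches DestroyTime.
; A Sphere1 overlap with a BPI_Damageable actor sends Damage through GetDamageMessage, prints a debug string and destroys the projectile.
; An older life-subtraction chain is left unconnected.
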(event `self.ReceiveTick`
  (params (DeltaSeconds :type "Float (single-precision)"))
  (`|ExecutionSequence`
    (:`then_0`
      (`self.K2_SetActorLocation` (+ (`self.K2_GetActorLocation`) (* (* (`self.GetActorForwardVector`) (`self.PushForce`)) DeltaSeconds))))
    (:`then_1`
      (set `self.DestroyCooldown` (+ (`self.DestroyCooldown`) DeltaSeconds))
      (if (>= (`self.DestroyCooldown`) (`self.DestroyTime`))
        (`self.K2_DestroyActor`)))))

(event `self.Sphere1.OnComponentBeginOverlap`
  (params (OverlappedComponent :type "PrimitiveComponent Object Reference") (OtherActor :type "Actor Object Reference") (OtherComp :type "PrimitiveComponent Object Reference") (OtherBodyIndex :type Integer) (bFromSweep :type Boolean) (SweepResult :type "HitResult Structure (by ref)"))
  (if (`KismetSystemLibrary.DoesImplementInterface` OtherActor "/Game/Blueprints/HP_BPs/Health/BPI_Damageable.BPI_Damageable_C")
    (message `/Game/Blueprints/HP_BPs/Health/BPI_Damageable.GetDamage` OtherActor (`self.Damage`))
    (`KismetSystemLibrary.PrintString` "Bullet Collision with damage Interface!" true true (struct :`R` 0.463182 :`B` 1.0 :`A` 1.0))
    (`self.K2_DestroyActor`)))

(fn `UserConstructionScript`)