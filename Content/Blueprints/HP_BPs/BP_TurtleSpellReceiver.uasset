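; Turtle puzzle actor that flips over during a timed vulnerable window, when it can be pushed with Flipendo.
; SetVulnerable, also called on BeginPlay, runs timers that blink VulnerableAlpha on two dynamic materials before the window ends.
; While vulnerable and off a pressure plate, Tick applies the flipped rotation and, when CanMove is set, sweeps it along PushDirection for PushDuration, up to MaxPushes.
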(event `SetVulnerable`
  (`KismetSystemLibrary.K2_ClearAndInvalidateTimerHandle` (`self.BlinkTimer`))
  (`KismetSystemLibrary.K2_ClearAndInvalidateTimerHandle` (`self.StartBlinkTimer`))
  (`KismetSystemLibrary.K2_ClearAndInvalidateTimerHandle` (`self.Endtimer`))
  (set `self.IsVulnerable` true)
  (set `self.CanUseFlipendo` true)
  (`self.SetVulnerableAlpha` 1.0)
  (bind _returnvalue (`KismetSystemLibrary.K2_SetTimerDelegate` (delegate `StartBlink`) (- (`self.VulnerableDuration`) (`self.BlinkStartBefore`))))
  (set `self.StartBlinkTimer` _returnvalue)
  (bind _returnvalue_2 (`KismetSystemLibrary.K2_SetTimerDelegate` (delegate `EndVulnerable`) (`self.VulnerableDuration`)))
  (set `self.Endtimer` _returnvalue_2))

(event `EndVulnerable`
  (`KismetSystemLibrary.K2_ClearAndInvalidateTimerHandle` (`self.BlinkTimer`))
  (set `self.IsVulnerable` false)
  (set `self.CanUseFlipendo` false)
  (set `self.BlinkOn` false)
  (`self.SetVulnerableAlpha` 0.0))

(event `StartBlink`
  (bind _returnvalue (`KismetSystemLibrary.K2_SetTimerDelegate` (delegate `ToggleBlink`) (`self.BlinkInterval`) true))
  (set `self.BlinkTimer` _returnvalue))

(event `ToggleBlink`
  (bind _blinkon (`self.BlinkOn`))
  (set `self.BlinkOn` (not _blinkon))
  (`self.SetVulnerableAlpha` (`KismetMathLibrary.SelectFloat` 1.0 0.0 _blinkon)))

(event `self.ReceiveBeginPlay`
  (bind _returnvalue (`PrimitiveComponent.CreateDynamicMaterialInstance` (`self.Cube`) 0 "/Game/M_Turtle.M_Turtle" "None"))
  (`KismetArrayLibrary.Array_Add` (`self.DynMats`) _returnvalue)
  (bind _returnvalue_2 (`PrimitiveComponent.CreateDynamicMaterialInstance` (`self.Cube1`) 0 "/Game/M_Turtle.M_Turtle" "None"))
  (`KismetArrayLibrary.Array_Add` (`self.DynMats`) _returnvalue_2)
  (`self.SetVulnerable`))

(event `self.ReceiveTick`
  (params (DeltaSeconds :type "Float (single-precision)"))
  (if (`self.IsOnPressurePlate`)
    _
    (elif (`self.CanUseFlipendo`)
      (`self.K2_SetActorRotation` (struct :`Yaw` 180.0 :`Roll` 180.0))
      (if (< (`self.currentPushes`) (`self.MaxPushes`))
        (if (`self.CanMove`)
          (set `self.CanObtainPlayerForward` true)
          (`|ExecutionSequence`
            (:`then_0`
              (`self.K2_SetActorLocation` (+ (`self.K2_GetActorLocation`) (* (* (stale _output_get_2) (`self.PushForce`)) DeltaSeconds)) true)
              (bind _output_get (set `self.pushCD` (+ (`self.pushCD`) (`GameplayStatics.GetWorldDeltaSeconds`))))
              (if (>= _output_get (`self.PushDuration`))
                (set `self.CanMove` false)
                (if (< (`self.currentPushes`) (`self.MaxPushes`))
                  (set `self.currentPushes` (+ (`self.currentPushes`) 1))
                  (set `self.pushCD` 0.0))))
            (:`then_1`
              (if (`self.CanObtainPlayerForward`)
                (bind _output_get_2 (set `self.PushDirection` (`self.SetPushDir`)))))
            (:`then_2`
              (set `self.CanObtainPlayerForward` false)))))
      (else
        (`self.K2_SetActorRotation` (struct :`Pitch` 180.0 :`Yaw` 180.0 :`Roll` 180.0))))))

(fn `SetVectorMove`
  (params (InputVector :type "Vector Structure")))

(fn `SetVulnerableAlpha`
  (params (Alpha :type "Float (double-precision)"))
  (for _array_element (`self.DynMats`)
    (`MaterialInstanceDynamic.SetScalarParameterValue` _array_element "VulnerableAlpha" (`local.Alpha`))))

(fn `UserConstructionScript`)