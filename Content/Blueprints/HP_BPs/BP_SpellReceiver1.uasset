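; BP_SpellReceiver1 is an actor that slides a limited number of times along its own axes, apparently as a pushable spell target.
; While CanMove is set, Tick moves it forward, back, right or left by MoveDirectionState at PushForce speed, without sweeping for collision.
; After PushDuration it stops and counts the push, ceasing to respond at MaxPushes.
; Nothing in this graph sets CanMove or the direction.
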(event `self.ReceiveTick`
  (params (DeltaSeconds :type "Float (single-precision)"))
  (if (< (`self.currentPushes`) (`self.MaxPushes`))
    (if (`self.CanMove`)
      (switch `/Game/Blueprints/Enums/Enum_SpellReciever_MoveDir` (`self.MoveDirectionState`)
        (:`NewEnumerator0`
          (`self.K2_SetActorLocation` (+ (`self.K2_GetActorLocation`) (* (* (`self.GetActorForwardVector`) (`self.PushForce`)) DeltaSeconds)))
          (bind _output_get (set `self.pushCD` (+ (`self.pushCD`) (`GameplayStatics.GetWorldDeltaSeconds`))))
          (if (>= _output_get (`self.PushDuration`))
            (set `self.CanMove` false)
            (if (< (`self.currentPushes`) (`self.MaxPushes`))
              (set `self.currentPushes` (+ (`self.currentPushes`) 1))
              (set `self.pushCD` 0.0))))
        (:`NewEnumerator1`
          (`self.K2_SetActorLocation` (+ (`self.K2_GetActorLocation`) (* (* (`KismetMathLibrary.NegateVector` (`self.GetActorForwardVector`)) (`self.PushForce`)) DeltaSeconds)))
          (bind _output_get_2 (set `self.pushCD` (+ (`self.pushCD`) (`GameplayStatics.GetWorldDeltaSeconds`))))
          (if (>= _output_get_2 (`self.PushDuration`))
            (set `self.CanMove` false)
            (if (< (`self.currentPushes`) (`self.MaxPushes`))
              (set `self.currentPushes` (+ (`self.currentPushes`) 1))
              (set `self.pushCD` 0.0))))
        (:`NewEnumerator2`
          (`self.K2_SetActorLocation` (+ (`self.K2_GetActorLocation`) (* (* (`self.GetActorRightVector`) (`self.PushForce`)) DeltaSeconds)))
          (bind _output_get_3 (set `self.pushCD` (+ (`self.pushCD`) (`GameplayStatics.GetWorldDeltaSeconds`))))
          (if (>= _output_get_3 (`self.PushDuration`))
            (set `self.CanMove` false)
            (if (< (`self.currentPushes`) (`self.MaxPushes`))
              (set `self.currentPushes` (+ (`self.currentPushes`) 1))
              (set `self.pushCD` 0.0))))
        (:`NewEnumerator3`
          (`self.K2_SetActorLocation` (+ (`self.K2_GetActorLocation`) (* (* (`KismetMathLibrary.NegateVector` (`self.GetActorRightVector`)) (`self.PushForce`)) DeltaSeconds)))
          (bind _output_get_4 (set `self.pushCD` (+ (`self.pushCD`) (`GameplayStatics.GetWorldDeltaSeconds`))))
          (if (>= _output_get_4 (`self.PushDuration`))
            (set `self.CanMove` false)
            (if (< (`self.currentPushes`) (`self.MaxPushes`))
              (set `self.currentPushes` (+ (`self.currentPushes`) 1))
              (set `self.pushCD` 0.0))))))))

(fn `UserConstructionScript`)