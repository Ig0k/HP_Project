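; BP_Door is a one-way sliding door that moves once its IsOpen flag is true; nothing in this Blueprint sets that flag.
; BeginPlay picks the slide direction from GoToRight, using the actor's forward vector or its negation.
; Tick moves the actor at OpenForce speed without sweep until the PushCd timer reaches MaxCd, and plays the opening sound once.
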(event `self.ReceiveBeginPlay`
  (if (`self.GoToRight`)
    (set `self.MoveDir` (`self.GetActorForwardVector`))
    (else
      (set `self.MoveDir` (`KismetMathLibrary.NegateVector` (`self.GetActorForwardVector`))))))

(event `self.ReceiveTick`
  (params (DeltaSeconds :type "Float (single-precision)"))
  (if (`self.IsOpen`)
    (`|ExecutionSequence`
      (:`then_0`
        (if (< (`self.PushCd`) (`self.MaxCd`))
          (`self.K2_SetActorLocation` (+ (`self.K2_GetActorLocation`) (* (* (`self.MoveDir`) (`self.OpenForce`)) DeltaSeconds)))
          (set `self.PushCd` (+ (`self.PushCd`) DeltaSeconds))))
      (:`then_1`
        (if (not (`self.SoundPlayed`))
          (`GameplayStatics.PlaySoundAtLocation` "/Game/Sounds/DoorOpenShortSFX.DoorOpenShortSFX" (`self.K2_GetActorLocation` self) (struct) 1.0 1.0 0.0 null null null null)
          (set `self.SoundPlayed` true))))))

(fn `UserConstructionScript`)