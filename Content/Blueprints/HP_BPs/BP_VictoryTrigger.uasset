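; BP_VictoryTrigger is a level-end trigger volume that fires when BP_HarryPotter overlaps its Box.
; The overlap sets Win, prints a win message and sets IsOpen on each valid BP_Door in its Doors array.
; A Sequence then opens the WIN level by object reference with no delay, while Tick reprints the message as long as Win is true.
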(event `self.ReceiveTick`
  (params (DeltaSeconds :type "Float (single-precision)"))
  (if (`self.Win`)
    (`KismetSystemLibrary.PrintString` "WIN LEVEL!" true true (struct :`G` 1.0 :`B` 0.119407 :`A` 1.0) 0.5)))

(event `self.Box.OnComponentBeginOverlap`
  (params (OverlappedComponent :type "PrimitiveComponent Object Reference") (OtherActor :type "Actor Object Reference") (OtherComp :type "PrimitiveComponent Object Reference") (OtherBodyIndex :type Integer) (bFromSweep :type Boolean) (SweepResult :type "HitResult Structure (by ref)"))
  (cast `/Game/ThirdPerson/Blueprints/BP_HarryPotter` OtherActor)
  (set `self.Win` true)
  (`|ExecutionSequence`
    (:`then_0`
      (`KismetSystemLibrary.PrintString` "WIN LEVEL!" true true (struct :`R` 0.076852 :`G` 1.0 :`A` 1.0) 10.0)
      (for _array_element (`self.Doors`)
        (if (`KismetSystemLibrary.IsValid` _array_element)
          (bind _asbp_door (cast `/Game/Blueprints/HP_BPs/BP_Door` _array_element))
          (if (not (`/Game/Blueprints/HP_BPs/BP_Door.IsOpen` _asbp_door))
            (set `/Game/Blueprints/HP_BPs/BP_Door.IsOpen` true _asbp_door)))))
    (:`then_1`
      (`GameplayStatics.OpenLevelBySoftObjectPtr` "/Game/WIN.WIN"))))

(fn `UserConstructionScript`)