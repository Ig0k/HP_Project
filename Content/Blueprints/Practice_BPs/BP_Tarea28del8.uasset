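; BP_Tarea28del8 is a practice Blueprint that randomly relocates the actors in its OtherActors array when play begins.
; On BeginPlay it shuffles the array and prints each actor's name and starting location on screen in red.
; It then reshuffles, offsets each actor by a random vector within fixed per-axis ranges without sweeping, and prints the new location in green.
; Tick, overlap and construction logic are empty.
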(event `self.ReceiveBeginPlay`
  (`KismetArrayLibrary.Array_Shuffle` (`self.OtherActors`))
  (bind _output_get (set `self.OtherActors` (`self.OtherActors`)))
  (for _array_element _output_get
    (`KismetSystemLibrary.PrintString` (`KismetStringLibrary.Concat_StrStr` "Actor " (`KismetSystemLibrary.GetDisplayName` _array_element) " START Position is: " (`KismetStringLibrary.Conv_VectorToString` (`self.K2_GetActorLocation` _array_element))) true true (struct :`R` 1.0 :`G` 0.035428 :`A` 1.0) 15.0))
  (`KismetArrayLibrary.Array_Shuffle` (`self.OtherActors`))
  (for (_array_element_2 _array_index) (`self.OtherActors`)
    (`self.K2_SetActorLocation` _array_element_2 (+ (`self.K2_GetActorLocation` _array_element_2) (`KismetMathLibrary.MakeVector` (`KismetMathLibrary.RandomFloatInRange` -500.0 800.0) (`KismetMathLibrary.RandomFloatInRange` 0.0 150.0) (`KismetMathLibrary.RandomFloatInRange` -500.0 800.0))) false false)
    (`KismetSystemLibrary.PrintString` (`KismetStringLibrary.Concat_StrStr` "Actor " (`KismetSystemLibrary.GetDisplayName` _array_element_2) " NEW Position is: " (`KismetStringLibrary.Conv_VectorToString` (`self.K2_GetActorLocation` _array_element_2))) true true (struct :`R` 0.362062 :`G` 1.0 :`A` 1.0) 15.0)))

(fn `UserConstructionScript`)