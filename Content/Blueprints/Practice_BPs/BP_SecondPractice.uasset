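; BP_SecondPractice is a practice Blueprint for learning loops, array operations and Branch conditionals.
; On BeginPlay it prints each index and value in the Names array, stopping when an element matches NameFind and printing a progress message otherwise.
; Disconnected example nodes show filling Names in a loop, setting CurrentLife from MaxLife, comparing the two, and basic array and comparison operators.
; Overlap, Tick and the construction script are empty.
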(event `self.ReceiveBeginPlay`
  ; Start
  (for (_array_element _array_index) (`self.Names`)
    (`KismetSystemLibrary.PrintString` (`KismetStringLibrary.Concat_StrStr` "Index: " (`KismetStringLibrary.Conv_IntToString` _array_index) " has Value: " _array_element) true true (struct :`R` 0.983755 :`G` 1.0 :`A` 1.0) 12.0)
    (if (`KismetStringLibrary.EqualEqual_StrStr` _array_element (`self.NameFind`))
      (break)
      (else
        (`KismetSystemLibrary.PrintString` "Recorriendo...")))))

(fn `UserConstructionScript`)