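; BP_ThirdPractice is a practice Blueprint for moving a list of actors by code.
; On BeginPlay it loops over the DifferentActors array, raises each actor 200 units from its current location, and prints the index and new location on screen.
; Two disconnected, commented examples contrast setting its own absolute location with adding an offset to it.
; Overlap, Tick and the construction script are empty.
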(event `self.ReceiveBeginPlay`
  ; Start
  (for (_array_element _array_index) (`self.DifferentActors`)
    (bind _returnvalue (`self.K2_GetActorLocation` _array_element))
    (`self.K2_SetActorLocation` _array_element (+ _returnvalue (0.0 0.0 200.0)) false false)
    (`KismetSystemLibrary.PrintString` (`KismetStringLibrary.Concat_StrStr` "Location actor " (`KismetStringLibrary.Conv_IntToString` _array_index) " is: " (`KismetStringLibrary.Conv_VectorToString` _returnvalue)) true true (struct :`G` 0.66 :`B` 1.0 :`A` 1.0) 10.0)))

(fn `UserConstructionScript`)