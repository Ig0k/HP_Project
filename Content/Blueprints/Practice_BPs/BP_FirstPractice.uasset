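; BP_FirstPractice is a practice actor that initializes a life value and prints a debug message.
; On BeginPlay it copies MaxLife into CurrentLife, then branches on DebuggVar.
; When true, it prints a Spanish greeting with its display name and life in a configurable color; otherwise it prints the flag's value.
; Overlap, Tick and the construction script are empty stubs, with the events labeled by Unity-style names.
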(event `self.ReceiveBeginPlay`
  (bind _debuggvar (`self.DebuggVar`))
  ; Start
  (bind _output_get (set `self.CurrentLife` (`self.MaxLife`)))
  (if _debuggvar
    (`KismetSystemLibrary.PrintString` (`KismetStringLibrary.Concat_StrStr` "Hola, " "Soy " (`KismetSystemLibrary.GetDisplayName` self) " y mi vida es: " (`KismetStringLibrary.Conv_DoubleToString` _output_get)) true true (`self.Text Color`))
    (else
      (`KismetSystemLibrary.PrintString` (`KismetStringLibrary.Concat_StrStr` "Debugging Var es: " (`KismetStringLibrary.Conv_BoolToString` _debuggvar))))))

(fn `UserConstructionScript`)